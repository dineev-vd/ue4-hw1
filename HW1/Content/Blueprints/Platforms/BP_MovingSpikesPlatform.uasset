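; Moving-spike platform that kills on contact, with the spike traveling along a spline.
; A timeline starting at a random time lerps distance along the spline to place the spike each update.
; Spike cycle duration shortens as game difficulty rises.
; Tick halves the timeline play rate while the boots bonus has time left, and spike collision overlap calls death.
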(event OnComponentBeginOverlap(SpikeCollision)
  (params (OverlappedComponent :type Primitive%20Component%20Object%20Reference) (OtherActor :type Actor%20Object%20Reference) (OtherComp :type Primitive%20Component%20Object%20Reference) (OtherBodyIndex :type Integer) (bFromSweep :type Boolean) (SweepResult :type Hit%20Result%20Structure%20%28by%20ref%29))
  (Default|CallDeath))

(event Custom|MoveSpike
  (bind _spline (Variables|Default|GetSpline))
  (bind _splinetimeline (Variables|Default|GetSplineTimeline))
  ;[1 1 1] We set timeline params here before its launch
  (Components|Timeline|SetPlayRate _splinetimeline (/ 1.0 (Variables|Default|GetDuration)))
  (Components|Timeline|SetNewTime _splinetimeline (Math|Random|RandomFloat))
  ;[1 1 1] As timeline plays, we set the position of spike according to position timeline gives us on the spline
  (bind _alpha (Timeline|SplineTimeline Play)
    (:Update
      (Variables|Default|SetAlpha _alpha)
      (Transformation|SetRelativeLocationAndRotation (Variables|Default|GetSpike) (Spline|GetLocationatDistanceAlongSpline _spline (Math|Float|Lerp 0.0 (Spline|GetSplineLength _spline) (Variables|Default|GetAlpha)) "Local") "0, 0, 0" false false))))

(event EventBeginPlay
  (|CallParentFunction)
  ;[1 1 1] Set the starting duration for spike and play animation
  (Variables|Default|SetDuration (+ (Variables|Default|GetBaseDuration) (/ 5.0 (Math|Conversions|ToFloat(Integer) (Variables|/Game/Blueprints/GameInstance/GI_Main.GI_Main_C|GetDifficulty (Variables|Default|GetGameInstance))))))
  (CallFunction|MoveSpike))

(event EventTick
  (params (DeltaSeconds :type Float%20%28single-precision%29))
  (bind _duration (Variables|Default|GetDuration))
  (bind _splinetimeline (Variables|Default|GetSplineTimeline))
  (if (> (Variables|/Game/Blueprints/GameInstance/GI_Main.GI_Main_C|GetBootsTimeLeft (Variables|Default|GetGameInstance)) 0.0)
    ;[1 1 1] We calculate the playrate and set it, according to active/inactive boots bonus
    (Components|Timeline|SetPlayRate _splinetimeline (/ 1.0 (* _duration 2.0)))
    (else
      (Components|Timeline|SetPlayRate _splinetimeline (/ 1.0 _duration))))
  (|CallParentFunction 0.0))

(fn ConstructionScript
  (|CallParentFunction))