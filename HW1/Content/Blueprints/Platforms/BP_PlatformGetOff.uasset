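; Platform with a knocker box that travels along a spline, apparently to push the player off.
; A timeline named Cart starts at a random time and drives the box's position along the spline while keeping its rotation, as the pillar mesh has an awkward pivot.
; Higher difficulty shortens the travel duration.
; Tick updates the play rate, halving the knocker's speed while the boots bonus is active.
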(event Custom|MoveKnocker
  (bind _knockerbox (Variables|Default|GetKnockerBox))
  (bind _spline (Variables|Default|GetSpline))
  (Components|Timeline|SetPlayRate (Variables|Default|GetCart) (/ 1.0 (Variables|Default|GetDuration)))
  (Components|Timeline|SetNewTime (Variables|Default|GetCart) (Math|Random|RandomFloat))
  (bind _alpha (Timeline|Cart Play)
    (:Update
      (Variables|Default|SetAlpha _alpha)
      (Transformation|SetRelativeLocationAndRotation _knockerbox (Spline|GetLocationatDistanceAlongSpline _spline (Math|Float|Lerp 0.0 (Spline|GetSplineLength _spline) (Variables|Default|GetAlpha)) "Local") (Variables|/Script/Engine.SceneComponent|GetRelativeRotation _knockerbox) false false))))

(event EventBeginPlay
  (|CallParentFunction)
  ;[1 1 1] Set the starting duration for knocker and play animation
  (Variables|Default|SetDuration (+ (Variables|Default|GetBaseDuration) (/ 5.0 (Math|Conversions|ToFloat(Integer) (Variables|/Game/Blueprints/GameInstance/GI_Main.GI_Main_C|GetDifficulty (Variables|Default|GetGameInstance))))))
  (CallFunction|MoveKnocker))

(event EventTick
  (params (DeltaSeconds :type Float%20%28single-precision%29))
  (bind _cart (Variables|Default|GetCart))
  (bind _duration (Variables|Default|GetDuration))
  (if (> (Variables|/Game/Blueprints/GameInstance/GI_Main.GI_Main_C|GetBootsTimeLeft (Variables|Default|GetGameInstance)) 0.0)
    ;[1 1 1] We calculate the playrate and set it, according to active/inactive boots bonus
    (Components|Timeline|SetPlayRate _cart (/ 1.0 (* _duration 2.0)))
    (else
      (Components|Timeline|SetPlayRate _cart (/ 1.0 _duration))))
  (|CallParentFunction 0.0))

(fn ConstructionScript
  (|CallParentFunction))