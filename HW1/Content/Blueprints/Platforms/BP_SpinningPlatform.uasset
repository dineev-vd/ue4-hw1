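; BP_SpinningPlatform is a platform that continuously spins its Floor component around the yaw axis.
; Each Tick it adds a frame-rate-independent yaw delta, using a base speed that rises linearly with the GameInstance Difficulty.
; While the GameInstance has BootsTimeLeft remaining, the rotation runs at half speed.
; BeginPlay, Tick and the construction script also call their parent implementations.
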(event EventBeginPlay
  (|CallParentFunction))

(event EventTick
  (params (DeltaSeconds :type Float%20%28single-precision%29))
  (bind _floor (Variables|Default|GetFloor))
  (bind _gameinstance (Variables|Default|GetGameInstance))
  (bind _floor_2 (Variables|Default|GetFloor))
  (bind _floor_3 (Variables|Default|GetFloor))
  (bind _returnvalue (Transformation|GetWorldRotation _floor_3))
  (bind _returnvalue_2 (Transformation|GetWorldRotation _floor_2))
  (bind _difficulty (Variables|/Game/Blueprints/GameInstance/GI_Main.GI_Main_C|GetDifficulty _gameinstance))
  (bind _returnvalue_3 (Math|Conversions|ToFloat(Integer) _difficulty))
  (bind _returnvalue_4 (* 30 _returnvalue_3))
  (bind _returnvalue_5 (+ 2e+01 _returnvalue_4))
  (bind _returnvalue_6 (* DeltaSeconds _returnvalue_5))
  (if (> (Variables|/Game/Blueprints/GameInstance/GI_Main.GI_Main_C|GetBootsTimeLeft (Variables|Default|GetGameInstance)) 0.0)
    ;[1 1 1] We rotate the platform with speed depending on Boots
    (Transformation|SetWorldRotation _floor (Math|Rotator|MakeRotator (.roll _returnvalue) (.pitch _returnvalue) (+ (.yaw _returnvalue) (* _returnvalue_6 0.5))) false false)
    (else
      (Transformation|SetWorldRotation _floor (Math|Rotator|MakeRotator (.roll _returnvalue_2) (.pitch _returnvalue_2) (+ (.yaw _returnvalue_2) (* _returnvalue_6 1.0))) false false)))
  (|CallParentFunction DeltaSeconds))

(fn ConstructionScript
  (|CallParentFunction))