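; BP_PlatformWall is a platform wall that becomes passable while the player's Boots pickup is active.
; Every Tick it reads BootsTimeLeft from the GameInstance.
; While time remains, it disables the Wall mesh's collision and swaps it for a visible transparent mesh.
; Otherwise it restores blocking collision and the solid mesh, then calls the parent Tick.
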(event EventBeginPlay
  (|CallParentFunction))

(event EventTick
  (params (DeltaSeconds :type Float%20%28single-precision%29))
  (bind _walltransparent (Variables|Default|GetWallTransparent))
  (bind _wall (Variables|Default|GetWall))
  (bind _wall_2 (Variables|Default|GetWall))
  (if (> (Variables|/Game/Blueprints/GameInstance/GI_Main.GI_Main_C|GetBootsTimeLeft (Variables|Default|GetGameInstance)) 0.0)
    ;[1 1 1] If Boots are picked up, the wall becomes transparent and has no collision, nice looking transparent mesh appears instead
    (Collision|SetCollisionProfileName _wall_2 "NoCollision" true :!class /Script/Engine.PrimitiveComponent)
    (Rendering|SetVisibility _walltransparent true false)
    (Rendering|SetVisibility _wall false false)
    (else
      (Collision|SetCollisionProfileName _wall_2 "BlockAll" true :!class /Script/Engine.PrimitiveComponent)
      (Rendering|SetVisibility _walltransparent false false)
      (Rendering|SetVisibility _wall true false)))
  (|CallParentFunction DeltaSeconds))

(fn ConstructionScript
  (|CallParentFunction))